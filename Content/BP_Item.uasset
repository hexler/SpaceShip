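; BP_Item is a moving pickup for the player spaceship, defined by an Item value holding a type and color.
; Its construction script creates a dynamic material on the mesh, which BeginPlay tints with the item's color.
; Tick moves it by Speed with sweep.
; Overlap with BP_SpaceShipPlayer plays a sound, calls the OnPickup dispatcher with item type and player, then removes the item through a very short lifespan.
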(event `self.ReceiveBeginPlay`
  (bind (_item_itemtype _item_color) (break `/Game/S_Item` (`self.Item`)))
  (`MaterialInstanceDynamic.SetVectorParameterValue` (`self.Material`) "Color" _item_color))

(event `self.ReceiveTick`
  (params (DeltaSeconds :type "Float (single-precision)"))
  (`self.K2_AddActorWorldOffset` (* (`self.Speed`) DeltaSeconds) true))

(event `self.ReceiveActorBeginOverlap`
  (params (OtherActor :type "Actor Object Reference"))
  (bind _item_itemtype (break `/Game/S_Item` (`self.Item`)))
  (bind _asbp_space_ship_player (cast `/Game/BP_SpaceShipPlayer` OtherActor))
  (`GameplayStatics.PlaySound2D` "/Engine/VREditor/Sounds/UI/Floating_UI_Close-001.Floating_UI_Close-001" 1.0 1.0 0.0 null null)
  (`self.OnPickup` _item_itemtype _asbp_space_ship_player)
  (`self.SetLifeSpan` 0.01))

(fn `UserConstructionScript`
  (bind _returnvalue (`PrimitiveComponent.CreateDynamicMaterialInstance` (`self.StaticMesh`) 0 null "None"))
  (set `self.Material` _returnvalue))