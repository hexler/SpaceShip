(event `self.ReceiveBeginPlay`
  (bind (_returnvalue_roll _returnvalue_pitch _returnvalue_yaw) (`KismetMathLibrary.BreakRotator` (`self.K2_GetActorRotation`)))
  (bind _initaillocation (`self.InitailLocation`))
  (bind _initialyaw (`self.InitialYaw`))
  ;[1 1 1] 事件开始
  (set `self.InitialYaw` _returnvalue_yaw)
  (set `self.InitailLocation` (`self.K2_GetActorLocation`))
  (set `self.CurrentHealth` (`self.MaxHealth`))
  ;[1 1 1] 出生动画 旋转
  (bind (_direction _movement_lerp) (`Timeline|SpawnAnime`)
    (:`Update`
      (`self.K2_SetActorLocation` (`KismetMathLibrary.VLerp` _initaillocation (+ _initaillocation (0.0 0.0 60.0)) _movement_lerp))
      (`self.K2_SetActorRotation` (`KismetMathLibrary.MakeRotator` 0.0 0.0 (`KismetMathLibrary.Lerp` _initialyaw (+ _initialyaw 720.0) _movement_lerp))))
    (:`Finished`
      (set `self.MovementEnable` true))))

(event `self.ReceiveTick`
  (params (DeltaSeconds :type "Float (single-precision)"))
  (if (`self.MovementEnable`)
    ;[1 1 1] 玩家角色进行移动
    (bind _output_get (set `self.CurrenrSpeed` (`KismetMathLibrary.FInterpTo` (`self.CurrenrSpeed`) (* DeltaSeconds (`self.GetInputAxisValue`) (`self.MoveSpeed`)) DeltaSeconds 4.0)))
    (`self.K2_AddActorWorldOffset` (`KismetMathLibrary.MakeVector` 0.0 _output_get) true)
    (`self.K2_SetActorRotation` (`KismetMathLibrary.MakeRotator` 0.0 0.0 (+ (`self.InitialYaw`) (* (`self.CurrenrSpeed`) -15.0))))))

(event `self.ReceiveAnyDamage`
  (params (Damage :type "Float (single-precision)") (DamageType :type "DamageType Object Reference") (InstigatedBy :type "Controller Object Reference") (DamageCauser :type "Actor Object Reference"))
  (`GameplayStatics.PlaySound2D` "/Engine/EditorSounds/GamePreview/EndSimulate_Cue.EndSimulate_Cue" 1.0 1.0 0.0 null null)
  (bind _output_get (set `self.CurrentHealth` (`KismetMathLibrary.FClamp` (- (`self.CurrentHealth`) Damage) 0.0 (`self.MaxHealth`))))
  (if (<= _output_get 0.0)
    (`self.SetLifeSpan` 0.02)))

(event `Fire`
  (`GameplayStatics.PlaySound2D` "/Engine/VREditor/Sounds/UI/Enter_Play.Enter_Play" 1.0 1.0 0.0 null null :!label _label)
  (`|SpawnActorFromClass` "/Game/BP_Bullet.BP_Bullet_C" (`self.GetTransform`) "Undefined" "OverrideRootScale" null 500.0 self (make `LinearColor` 1.0 0.0 0.0 1.0) null))

(event `Key|LeftMouseButton`
  (params (Key :type "Key Structure"))
  (:`Pressed`
    (`KismetSystemLibrary.K2_SetTimerDelegate` (delegate `Fire`) 0.3 true)
    (goto _label))
  (:`Released`
    (`KismetSystemLibrary.K2_ClearTimer` null "Fire")))

(event `self.ReceiveDestroyed`
  (`GameplayStatics.SpawnEmitterAtLocation` "/Game/Arts/Particles/P_Pixel_Explosion_Player.P_Pixel_Explosion_Player" (`self.K2_GetActorLocation`)))

(fn `UserConstructionScript`)