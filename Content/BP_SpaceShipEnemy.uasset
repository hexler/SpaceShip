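; Enemy spaceship that spins into place on spawn, then descends along -Z while strafing on Y and shooting at the player.
; A randomized Delay in Tick throttles fire, spawning BP_Bullet when the player is roughly aligned on Y.
; Hitting the player deals damage and destroys the ship, while other hits reverse its strafe.
; Damage updates health and its status widget, destroying the ship at zero with explosion and sound.
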(event `self.ReceiveBeginPlay`
  (bind (_returnvalue_roll _returnvalue_pitch _returnvalue_yaw) (`KismetMathLibrary.BreakRotator` (`self.K2_GetActorRotation`)))
  (bind _initaillocation (`self.InitailLocation`))
  (bind _initialyaw (`self.InitialYaw`))
  ;[1 1 1] 事件开始
  (set `self.InitialYaw` _returnvalue_yaw)
  (set `self.InitailLocation` (`self.K2_GetActorLocation`))
  (set `self.CurrentHealth` (`self.MaxHealth`))
  ;[1 1 1] 出生动画 旋转
  (bind (_direction _movement_lerp) (`Timeline|SpawnAnime`)
    (:`Update`
      (`self.K2_SetActorLocation` (`KismetMathLibrary.VLerp` _initaillocation (+ _initaillocation (0.0 0.0 -60.0)) _movement_lerp))
      (`self.K2_SetActorRotation` (`KismetMathLibrary.MakeRotator` 0.0 0.0 (`KismetMathLibrary.Lerp` _initialyaw (+ _initialyaw 720.0) _movement_lerp))))
    (:`Finished`
      (set `self.MovementEnable` true))))

(event `self.ReceiveTick`
  (params (DeltaSeconds :type "Float (single-precision)"))
  (bind _returnvalue (`GameplayStatics.GetPlayerPawn` 0))
  (if (`self.MovementEnable`)
    ;[1 1 1] 敌方角色进行移动
    (`self.K2_AddActorWorldOffset` (* (`KismetMathLibrary.MakeVector` 0.0 (* (`self.MoveSpeed`) (`KismetMathLibrary.SelectFloat` -1.0 1.0 (`self.MovementDirection`))) -45.0) DeltaSeconds) true)
    (`/Engine/EditorBlueprintResources/StandardMacros.IsValid` _returnvalue
      (:`Is Valid`
        (`KismetSystemLibrary.Delay` (`KismetMathLibrary.RandomFloatInRange` 0.4 0.6))
        (`/Engine/EditorBlueprintResources/StandardMacros.IsValid` _returnvalue
          (:`Is Valid`
            (if (<= (`KismetMathLibrary.VSize` (* (- (`self.K2_GetActorLocation` _returnvalue) (`self.K2_GetActorLocation`)) (0.0 1.0 0.0))) 80.0)
              (`|SpawnActorFromClass` "/Game/BP_Bullet.BP_Bullet_C" (`self.GetTransform`) "Undefined" "OverrideRootScale" null -300.0 self (make `LinearColor` 0.0 1.0 0.0 1.0) null))))))))

(event `self.ReceiveHit`
  (params (MyComp :type "PrimitiveComponent Object Reference") (Other :type "Actor Object Reference") (OtherComp :type "PrimitiveComponent Object Reference") (bSelfMoved :type Boolean) (HitLocation :type "Vector Structure") (HitNormal :type "Vector Structure") (NormalImpulse :type "Vector Structure") (Hit :type "HitResult Structure (by ref)"))
  (bind _asbp_space_ship_player (cast `/Game/BP_SpaceShipPlayer` Other)
    (:`then`
      (`GameplayStatics.ApplyDamage` _asbp_space_ship_player 80.0)
      (`self.K2_DestroyActor`))
    (:`CastFailed`
      (set `self.MovementDirection` (not (`self.MovementDirection`))))))

(event `self.ReceiveAnyDamage`
  (params (Damage :type "Float (single-precision)") (DamageType :type "DamageType Object Reference") (InstigatedBy :type "Controller Object Reference") (DamageCauser :type "Actor Object Reference"))
  (`GameplayStatics.PlaySound2D` "/Engine/VREditor/Sounds/UI/Click_on_Button_Cue.Click_on_Button_Cue" 1.0 1.0 0.0 null null)
  (bind _output_get (set `self.CurrentHealth` (`KismetMathLibrary.FClamp` (- (`self.CurrentHealth`) Damage) 0.0 (`self.MaxHealth`))))
  (`self.SyncHealth`)
  (if (<= _output_get 0.0)
    (`self.K2_DestroyActor`)))

(event `self.ReceiveDestroyed`
  (`GameplayStatics.SpawnEmitterAtLocation` "/Game/Arts/Particles/P_Pixel_Explosion_Enemy.P_Pixel_Explosion_Enemy" (`self.K2_GetActorLocation`))
  (`GameplayStatics.PlaySound2D` "/Engine/EditorSounds/Notifications/CompileSuccess_Cue.CompileSuccess_Cue" 1.0 1.0 0.0 null null)
  (`self.K2_DestroyActor`))

(fn `SyncHealth`
  (bind _aswb_enemy_status (cast `/Game/Arts/UI/WB_Enemy_Status` (`WidgetComponent.GetUserWidgetObject` (`self.Widget`))))
  (`/Game/Arts/UI/WB_Enemy_Status.SetHealth` _aswb_enemy_status (`KismetMathLibrary.FTrunc` (`self.CurrentHealth`)) (`KismetMathLibrary.FTrunc` (`self.MaxHealth`))))

(fn `UserConstructionScript`)