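; BP_GameController runs a spaceship game's loop, owning the fixed camera, spawn points, lives and status widget.
; It spawns and possesses the player, syncing health on damage; death shakes the camera by timeline, clears enemies, then respawns or shows game over.
; A gated Tick with random Delay spawns enemies at varied Y positions, and a trigger destroys those reaching it.
; Destroyed enemies may drop health or life pickups.
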(event `GameOver`
  (bind _returnvalue (`GameplayStatics.GetPlayerController` 0))
  ;[1 1 1] 游戏结束
  (`GameplayStatics.PlaySound2D` "/Engine/VREditor/Sounds/VR_click1.VR_click1" 1.0 1.0 0.0 null null)
  (bind _returnvalue_2 (`|CreateWidget` "/Game/Arts/UI/WB_GameOver.WB_GameOver_C" null self))
  (`UserWidget.AddToViewport` _returnvalue_2 0)
  (set `PlayerController.bShowMouseCursor` true _returnvalue)
  (`WidgetBlueprintLibrary.SetInputMode_GameAndUIEx` _returnvalue _returnvalue_2 "LockInFullscreen"))

(event `self.Trigger.OnComponentBeginOverlap`
  (params (OverlappedComponent :type "PrimitiveComponent Object Reference") (OtherActor :type "Actor Object Reference") (OtherComp :type "PrimitiveComponent Object Reference") (OtherBodyIndex :type Integer) (bFromSweep :type Boolean) (SweepResult :type "HitResult Structure (by ref)"))
  ;[1 1 1] 地图的碰撞
  (if (`KismetArrayLibrary.Array_Contains` (`self.enemies`) OtherActor)
    (`self.K2_DestroyActor` OtherActor)))

(event `self.ReceiveBeginPlay`
  ;[1 1 1] 游戏开始操作
  (`self.SpawnPlayer`)
  (`self.StartSpawnEnemy`)
  (`WidgetBlueprintLibrary.SetInputMode_GameOnly` (`GameplayStatics.GetPlayerController` 0))
  (set `self.GameRunning` true))

(event `PlaySnake`
  (params (intenstiy :type "Float (double-precision)"))
  ;[1 1 1] 相机震动
  (bind (_direction _movementlerp) (`Timeline|CamraSnake` :!via `PlayFromStart`)
    (:`Update`
      (`SceneComponent.K2_SetRelativeLocation` (`self.Camera`) (* _movementlerp intenstiy) true false))))

(event `ReSpawn`
  ;[1 1 1] 重生
  (`self.SpawnPlayer`)
  (set `self.GameRunning` true)
  (`self.StartSpawnEnemy`))

(event `SpawnPlayer`
  (bind _returnvalue (`GameplayStatics.GetPlayerController` 0))
  ;[1 1 1] 生成玩家角色
  (`self.SyncLife`)
  (bind _returnvalue_2 (`|SpawnActorFromClass` "/Game/BP_SpaceShipPlayer.BP_SpaceShipPlayer_C" (`SceneComponent.K2_GetComponentToWorld` (`self.SpawnPointPlayer`)) "AdjustIfPossibleButAlwaysSpawn" "OverrideRootScale" null null))
  (`Controller.Possess` _returnvalue _returnvalue_2)
  (`PlayerController.SetViewTargetWithBlend` _returnvalue self 0.0 "VTBlend_Linear" 0.0 false)
  ;[1 1 1] 死亡事件
  (add `self.OnDestroyed` _returnvalue_2 (delegate `OnPlayerKilled`))
  ;[1 1 1] 伤害血条同步
  (`self.SyncHealth` _returnvalue_2)
  (add `self.OnTakeAnyDamage` _returnvalue_2 (delegate `OnPlayerDamaged`)))

(event `OnPlayerKilled` :!signature `self.OnDestroyed`
  (params (DestroyedActor :type "Actor Object Reference"))
  ;[1 1 1] 死亡事件
  (`PlayerController.SetViewTargetWithBlend` (`GameplayStatics.GetPlayerController` 0) self 0.0 "VTBlend_Linear" 0.0 false)
  (`self.PlaySnake` -5.0)
  (set `self.GameRunning` false)
  (`self.StopSpawnEnemy`)
  (`KismetSystemLibrary.Delay` 3.0)
  (bind _isdead (`self.IsGameOver`))
  (if _isdead
    (`self.GameOver`)
    (else
      (`self.DecreaseLife`)
      (`self.ReSpawn`))))

(event `OnPlayerDamaged` :!signature `self.OnTakeAnyDamage`
  (params (DamagedActor :type "Actor Object Reference") (Damage :type "Float (double-precision)") (DamageType :type "DamageType Object Reference") (InstigatedBy :type "Controller Object Reference") (DamageCauser :type "Actor Object Reference"))
  ;[1 1 1] 伤害血条同步
  (`self.SyncHealth` DamagedActor))

(event `SpawnEnemy`
  (bind _spawnrange (`self.SpawnRange`))
  (bind (_returnvalue_location _returnvalue_rotation _returnvalue_scale) (`KismetMathLibrary.BreakTransform` (`SceneComponent.K2_GetComponentToWorld` (`self.SpawnPointEnemy`))))
  ;[1 1 1] 生成敌人
  (if (and (`self.EnableSpawnEnemy`) (`self.GameRunning`))
    (bind _returnvalue (`|SpawnActorFromClass` "/Game/BP_SpaceShipEnemy.BP_SpaceShipEnemy_C" (`KismetMathLibrary.MakeTransform` (`KismetMathLibrary.MakeVector` (.x _returnvalue_location) (+ (`KismetMathLibrary.RandomFloatInRange` _spawnrange (* _spawnrange -1.0)) (.y _returnvalue_location)) (.z _returnvalue_location)) _returnvalue_rotation _returnvalue_scale) "AdjustIfPossibleButAlwaysSpawn" "OverrideRootScale" null 80.0 null))
    (`KismetArrayLibrary.Array_Add` (`self.enemies`) _returnvalue)
    ;[1 1 1] 敌人死亡处理
    (add `self.OnDestroyed` _returnvalue (delegate `OnEnemyKilled`))))

(event `OnEnemyKilled` :!signature `self.OnDestroyed`
  (params (DestroyedActor :type "Actor Object Reference"))
  ;[1 1 1] 敌人死亡处理
  (`KismetArrayLibrary.Array_RemoveItem` (`self.enemies`) DestroyedActor)
  (`self.ProcessItemDrop` DestroyedActor))

(event `ProcessItemDrop`
  (params (Target :type "Actor Object Reference"))
  ;[1 1 1] 道具生成
  (if (`self.GameRunning`)
    (if (< (`KismetMathLibrary.RandomInteger` 5) 1)
      (bind _returnvalue (`|SpawnActorFromClass` "/Game/BP_Item.BP_Item_C" (`self.GetTransform` Target) "Undefined" "OverrideRootScale" null (`|GetArrayItem` (`self.Item`) (`KismetMathLibrary.RandomInteger` (`KismetArrayLibrary.Array_Length` (`self.Item`)))) null))
      (add `/Game/BP_Item.OnPickup` _returnvalue (delegate `OnpickupItem`)))))

(event `OnpickupItem`
  (params (ItemType :type "/Game/E_Item Enum" :default "NewEnumerator0") (Actor :type "Actor Object Reference"))
  ;[1 1 1] 道具生成
  (switch `/Game/E_Item` ItemType
    (:`NewEnumerator1`
      (`GameplayStatics.ApplyDamage` Actor -10.0))
    (:`NewEnumerator2`
      (`self.IncreaseLife` 1))))

(event `self.ReceiveTick`
  (params (DeltaSeconds :type "Float (single-precision)"))
  ;[1 1 1] 敌人生成规则
  (`/Engine/EditorBlueprintResources/StandardMacros.Gate` true :!label _label
    (:`Exit`
      (`KismetSystemLibrary.Delay` (`KismetMathLibrary.RandomFloatInRange` 3.5 5.0))
      (`self.SpawnEnemy`))))

(event `StartSpawnEnemy`
  ;[1 1 1] 敌人生成规则
  (set `self.EnableSpawnEnemy` true)
  (goto _label :!via `Open`))

(event `StopSpawnEnemy`
  (bind _enemiesdelete (`self.enemiesDelete`))
  ;[1 1 1] 敌人生成规则
  (set `self.EnableSpawnEnemy` false)
  (for _array_element (`self.enemies`)
    (`KismetArrayLibrary.Array_Add` _enemiesdelete _array_element))
  (for _array_element_2 _enemiesdelete
    (`self.K2_DestroyActor` _array_element_2))
  (`KismetArrayLibrary.Array_Clear` _enemiesdelete)
  (goto _label :!via `Close`))

(fn `DecreaseLife`
  (`/Engine/EditorBlueprintResources/StandardMacros.DecrementInt` (`self.Life`)))

(fn `IncreaseLife`
  (params (Value :type Integer))
  (set `self.Life` (+ Value (`self.Life`)))
  (`self.SyncLife`))

(fn `IsGameOver`
  (returns (IsDead :type Boolean))
  (return (< (`self.Life`) 1)))

(fn `QuitGame`
  (set `self.GameRunning` false)
  (`KismetSystemLibrary.QuitGame` null "Quit"))

(fn `ReStart`
  (set `self.GameRunning` true)
  (`GameplayStatics.OpenLevel` "GameLevel"))

(fn `SyncHealth`
  (params (Player :type "Actor Object Reference"))
  (bind _asbp_space_ship_player (cast `/Game/BP_SpaceShipPlayer` Player))
  (`/Game/Arts/UI/WB_Play_Status.SetHealth` (cast `/Game/Arts/UI/WB_Play_Status` (`WidgetComponent.GetUserWidgetObject` (`self.PlayerStatus`)) :!pure true) (/ (`/Game/BP_SpaceShipPlayer.CurrentHealth` _asbp_space_ship_player) (`/Game/BP_SpaceShipPlayer.MaxHealth` _asbp_space_ship_player))))

(fn `SyncLife`
  (`/Game/Arts/UI/WB_Play_Status.SetLife` (cast `/Game/Arts/UI/WB_Play_Status` (`WidgetComponent.GetUserWidgetObject` (`self.PlayerStatus`)) :!pure true) (`self.Life`)))

(fn `UserConstructionScript`
  (`SceneComponent.K2_SetRelativeLocation` (`self.SpawnPointPlayer`) (`self.SpawnLocationPlayer`) false false)
  (`SceneComponent.K2_SetRelativeLocation` (`self.SpawnPointEnemy`) (`self.SpawnLocationEnemy`) false false)
  (`SceneComponent.K2_SetRelativeLocation` (`self.Trigger`) (`self.SpawnLocationTrigger`) false false)
  (`SceneComponent.K2_SetRelativeLocation` (`self.PlayerStatus`) (`self.SpawnLocationPlayerStatus`) false false))