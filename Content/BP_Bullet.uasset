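; BP_Bullet is a projectile actor that moves along world Z at MoveSpeed and damages what it hits.
; The construction script creates a dynamic material instance on the Bullet component, which BeginPlay tints with the Color variable.
; Tick applies the frame-rate independent offset.
; On overlapping any actor other than MyCreator, it applies fixed damage and destroys itself.
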(event `self.ReceiveBeginPlay`
  (`MaterialInstanceDynamic.SetVectorParameterValue` (`self.Material`) "Color2" (`self.Color`)))

(event `self.ReceiveTick`
  (params (DeltaSeconds :type "Float (single-precision)"))
  (`self.K2_AddActorWorldOffset` (`KismetMathLibrary.MakeVector` 0.0 0.0 (* (`self.MoveSpeed`) DeltaSeconds))))

(event `self.ReceiveActorBeginOverlap`
  (params (OtherActor :type "Actor Object Reference"))
  (if (!= (`self.MyCreator`) OtherActor)
    (`GameplayStatics.ApplyDamage` OtherActor 20.0)
    (`self.K2_DestroyActor`)))

(fn `UserConstructionScript`
  (bind _returnvalue (`PrimitiveComponent.CreateDynamicMaterialInstance` (`self.Bullet`) 0 null "None"))
  (set `self.Material` _returnvalue))